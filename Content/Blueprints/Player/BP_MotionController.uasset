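; BP_MotionController is a player motion controller with an animated hand mesh that reflects grip state.
; Each tick it sets a three-value GripState from whether an actor is attached or grip is wanted, whether a grabbable candidate is near the hand, or neither.
; It then copies that state to the hand mesh's RightHand_AnimBP to drive the pose.
; This graph contains no grab, release or input logic.
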(event `self.ReceiveTick`
  (params (DeltaSeconds :type "Float (single-precision)"))
  (`|ExecutionSequence`
    (:`then_0`
      ;[1 1 1] Update Grip State Enum
      (if (or (!= (`self.AttachedActor`) null) (`self.bWantsToGrip`))
        (set `self.GripState` "NewEnumerator2")
        (else
          (bind _returnvalue (`self.GetActorNearHand`))
          (if (!= _returnvalue null)
            (set `self.GripState` "NewEnumerator1")
            (elif (`self.bWantsToGrip`)
              (set `self.GripState` "NewEnumerator2")
              (else
                (set `self.GripState` "NewEnumerator0")))))))
    (:`then_1`
      ;[1 1 1] Update animation state of hand mesh
      (bind _asright_hand_anim_bp (cast `/Game/VirtualReality/Mannequin/Animations/RightHand_AnimBP` (`SkeletalMeshComponent.GetAnimInstance` (`self.ControllerHandMesh`))))
      (set `/Game/VirtualReality/Mannequin/Animations/RightHand_AnimBP.GripState` (`self.GripState`) _asright_hand_anim_bp))))

(fn `UserConstructionScript`)