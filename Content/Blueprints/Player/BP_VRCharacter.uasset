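; BP_VRCharacter is the VR player character, handling UI pointer clicks, turning and a toggleable in-world menu.
; Left and right select inputs press and release left mouse on each hand's interaction component, while OpenMenu spawns BP_VRMenu attached to MenuLoc or destroys it.
; The Turn axis rotates VRRoot around the camera position rather than the capsule.
; A TEST input fires left-hand haptics; tracking-origin, movement and broken snap-turn logic are unconnected.
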(event `self.ReceiveBeginPlay`)

(event `InputAction|LeftSelect`
  (params (Key :type "Key Structure"))
  (bind _leftinteractioncomp (`self.LeftInteractionComp`))
  (:`Pressed`
    (`WidgetInteractionComponent.PressPointerKey` _leftinteractioncomp "LeftMouseButton"))
  (:`Released`
    (`WidgetInteractionComponent.ReleasePointerKey` _leftinteractioncomp "LeftMouseButton")))

(event `InputAction|RightSelect`
  (params (Key :type "Key Structure"))
  (bind _rightinteractioncomp (`self.RightInteractionComp`))
  (:`Pressed`
    (`WidgetInteractionComponent.PressPointerKey` _rightinteractioncomp "LeftMouseButton"))
  (:`Released`
    (`WidgetInteractionComponent.ReleasePointerKey` _rightinteractioncomp "LeftMouseButton")))

(event `InputAction|OpenMenu`
  (params (Key :type "Key Structure"))
  (:`Pressed`
    (`self.Create Menu`)))

(event `InputAxis|Turn`
  (params (AxisValue :type "Float (single-precision)"))
  (bind _vrroot (`self.VRRoot`))
  (bind _returnvalue (`SceneComponent.K2_GetComponentLocation` (`self.VRCameraComp`)))
  ;[1 1 1] Rotation around current camera position - not capsule pos
  (`SceneComponent.K2_SetWorldLocation` _vrroot (+ (`KismetMathLibrary.RotateAngleAxis` (- (`SceneComponent.K2_GetComponentLocation` (`self.VRRoot`)) _returnvalue) AxisValue (0.0 0.0 1.0)) _returnvalue) false false)
  (`SceneComponent.K2_AddRelativeRotation` _vrroot (`KismetMathLibrary.MakeRotator` 0.0 0.0 AxisValue) false false))

(event `InputAction|TEST`
  (params (Key :type "Key Structure"))
  (:`Pressed`
    (`PlayerController.PlayHapticEffect` (`GameplayStatics.GetPlayerController` 0) "/Game/Haptics/VRControllerHaptic.VRControllerHaptic" "Left" 1.0 false)))

(fn `Create Menu`
  (bind _vrmenu (`self.VRMenu`))
  (`/Engine/EditorBlueprintResources/StandardMacros.IsValid` _vrmenu
    (:`Is Valid`
      (`self.K2_DestroyActor` _vrmenu)
      (set `self.VRMenu` null))
    (:`Is Not Valid`
      (bind _returnvalue (`|SpawnActorFromClass` "/Game/Blueprints/HUD/BP_VRMenu.BP_VRMenu_C" (`KismetMathLibrary.MakeTransform` (0.0 0.0 0.0) (struct) (0.5 0.5 0.5)) "Undefined" "OverrideRootScale" null null))
      (bind _output_get (set `self.VRMenu` _returnvalue))
      (`self.K2_AttachToComponent` _output_get (`self.MenuLoc`) "None" "SnapToTarget" "SnapToTarget" "KeepWorld" true)
      (`SceneComponent.K2_SetRelativeRotation` (`Actor.RootComponent` _output_get) (struct :`Yaw` 180.0) false false)
      (`KismetSystemLibrary.PrintString` "Opening Menu!" true true (struct :`G` 0.66 :`B` 1.0 :`A` 1.0) 3.0))))

(fn `UserConstructionScript`)